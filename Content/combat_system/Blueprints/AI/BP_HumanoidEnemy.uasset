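; BP_HumanoidEnemy is a humanoid enemy Blueprint in the combat system that adds a targeting-driven health bar to its parent's behavior.
; On BeginPlay it creates a WB_HealthBar widget bound to its own StatsComponent, assigns it to the Healthbar component and hides it.
; OnTargeted shows or hides the bar with the targeting state, while construction and CanBeTargeted simply defer to the parent.
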(event `self.ReceiveBeginPlay`
  (`parent.ReceiveBeginPlay`)
  (bind _returnvalue (`|CreateWidget` "/Game/combat_system/UI/WB_HealthBar.WB_HealthBar_C" (`GameplayStatics.GetPlayerController` 0) (`self.StatsComponent`) false))
  (`WidgetComponent.SetWidget` (`self.Healthbar`) _returnvalue)
  (`SceneComponent.SetVisibility` (`self.Healthbar`) false false))

(event `/Game/combat_system/Blueprints/Interfaces/Targetable_BPI.OnTargeted`
  (params (isTargeted :type Boolean))
  (`parent.OnTargeted` isTargeted)
  (`SceneComponent.SetVisibility` (`self.Healthbar`) isTargeted false))

(fn `CanBeTargeted`
  (returns (`canBe Targeted` :type Boolean))
  (bind _canbe_targeted (`parent.CanBeTargeted`))
  (return _canbe_targeted))

(fn `UserConstructionScript`
  (`parent.UserConstructionScript`))