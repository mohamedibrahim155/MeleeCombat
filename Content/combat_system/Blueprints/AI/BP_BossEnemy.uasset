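; Boss enemy Blueprint that extends a parent AI combat character with a dedicated boss health bar and a physical weapon.
; On BeginPlay it creates the health widget from its StatsComponent, showing it when the AI sees a valid actor and hiding it on death.
; Weapon collision hits apply stat-based point damage to damageable actors.
; Combat toggles move the weapon between sockets, and death switches it to physics simulation.
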(event `self.ReceiveBeginPlay`
  (bind _bosshealtthui (`self.BossHealtthUI`))
  (`parent.ReceiveBeginPlay`)
  (`/Game/combat_system/Blueprints/Components/CollisionComponent.SetMeshComponent` (`self.MainWeaponCollisionComponent`) (`self.WeaponMesh`))
  (bind _returnvalue (`|CreateWidget` "/Game/combat_system/UI/WB_BossHealth.WB_BossHealth_C" (`GameplayStatics.GetPlayerController` 0)))
  (set `self.BossHealtthUI` _returnvalue)
  (`/Game/combat_system/UI/WB_BossHealth.Initilise` _bosshealtthui (`self.StatsComponent`))
  (`UserWidget.AddToViewport` _bosshealtthui 0))

(event `self.OnTargeted`
  (params (isTargeted :type Boolean))
  ;[1 0 0.02291] On targeted
  (`parent.OnTargeted` isTargeted))

(event `self.MainWeaponCollisionComponent.OnHit`
  (params (hitInfo :type "HitResult Structure"))
  (bind (_bblockinghit _binitialoverlap _time _distance _location _impactpoint _normal _impactnormal _physmat _hitactor) (`GameplayStatics.BreakHitResult` hitInfo))
  (bind _returnvalue (`self.GetOwner`))
  (bind _returrnvalue (`/Game/combat_system/Blueprints/Components/StatsComponent.GetCurrentStatValue` (`self.StatsComponent`) "NewEnumerator4"))
  ;[1 0 0.01335] On Hit
  (bind _returnvalue_2 (message `/Game/combat_system/Blueprints/Interfaces/ContinueAttack_BPI.CanReceiveDamage` _hitactor))
  (if (and _returnvalue_2 (!= _hitactor _returnvalue))
    (`KismetSystemLibrary.PrintString` (`KismetStringLibrary.Conv_DoubleToString` _returrnvalue) true true (struct :`R` 1.0 :`G` 0.966577 :`A` 1.0))
    (`GameplayStatics.ApplyPointDamage` _hitactor _returrnvalue (`self.GetActorForwardVector` _returnvalue) hitInfo (`self.GetController`) _returnvalue "/Game/combat_system/Blueprints/DamageTypes/BP_AttackDamageType.BP_AttackDamageType_C")))

(event `SimulateWeaponPhysics`
  (bind _weaponmesh (`self.WeaponMesh`))
  ;[1 0.01374 0] Simulate AI's Weapon
  (`PrimitiveComponent.SetCollisionProfileName` _weaponmesh "PhysicsActor" true)
  (`PrimitiveComponent.SetSimulatePhysics` _weaponmesh true))

(event `self.PerformDead`
  ;[1 0 0] AI dead
  (`parent.PerformDead`)
  (`self.SimulateWeaponPhysics`)
  (`self.SetBossHealthVisivbility` false))

(event `self.CombatComponent.OnToggleCombat`
  (params (`is Combat Enabled` :type Boolean))
  ;[1 1 1] OnToggleCombat
  (`SceneComponent.K2_AttachToComponent` (`self.WeaponMesh`) (`self.Mesh`) (select `bool` `is Combat Enabled` :`false` (`self.Attach Socket Name`) :`true` (`self.WeaponAttachSocketName`)) "SnapToTarget" "SnapToTarget" "SnapToTarget" true))

(event `self.ToggleCombat`
  (`parent.ToggleCombat`))

(event `SetBossHealthVisivbility`
  (params (isVisible :type Boolean))
  ;[1 0.006082 0] SetBossHealth Active state
  (bind _bosshealtthui (`self.BossHealtthUI`)
    (:`then`
      (`Widget.SetVisibility` _bosshealtthui (select `bool` isVisible :`false` "Hidden" :`true` "Visible" :!type "ESlateVisibility Enum")))
    (:`else`)))

(event `self.OnSeenActor`
  (params (`Seen Actor` :type "Actor Object Reference"))
  ;[1 0 0.03079] TargetSet from AI controller
  (`parent.OnSeenActor` `Seen Actor`)
  (`self.SetBossHealthVisivbility` (`KismetSystemLibrary.IsValid` `Seen Actor`))
  (`KismetSystemLibrary.PrintString` "Wokring" true true (struct :`G` 1.0 :`B` 0.14433 :`A` 1.0)))

(fn `CanBeTargeted`
  (returns (`canBe Targeted` :type Boolean))
  (bind _canbe_targeted (`parent.CanBeTargeted`))
  (return _canbe_targeted))

(fn `Perform Combat Action`
  (params (StateTag :type "GameplayTag Structure") (ActionTag :type "GameplayTag Structure") (MontageIndex :type Integer) (bIsRandomIndex :type Boolean))
  (returns (`action Duration` :type "Float (double-precision)"))
  (bind _action_duration (`parent.Perform Combat Action` StateTag ActionTag MontageIndex bIsRandomIndex))
  (return _action_duration))

(fn `Perform Combat Attack`
  (params (AttackTypeTag :type "GameplayTag Structure") (AttackCount :type Integer) (bIsRandomAttack :type Boolean))
  (returns (`Attack Duration` :type "Float (double-precision)"))
  (bind _attack_duration (`parent.Perform Combat Attack` AttackTypeTag AttackCount bIsRandomAttack))
  (return _attack_duration))

(fn `UserConstructionScript`
  (`parent.UserConstructionScript`))