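; BP_CharacterTest is a test character for the combat system that can be a lock-on target.
; On BeginPlay it initialises its StatsComponent, then spawns and equips each class in Armours, printing a current stat value after each piece.
; Being targeted toggles its LockOnWidget, and CanBeTargeted refuses targeting when the StateManagerComponent reports the Dead state.
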(event `self.ReceiveBeginPlay`
  (`/Game/combat_system/Blueprints/Components/StatsComponent.IntialiseStats` (`self.StatsComponent`))
  (for _array_element (`self.Armours`)
    (bind _returnvalue (`|SpawnActorFromClass` _array_element (`self.GetTransform`) "Undefined" "MultiplyWithRoot" self self))
    (`/Game/combat_system/Blueprints/Actors/BP_BaseEquippaable.OnEquipped` _returnvalue)
    (`KismetSystemLibrary.PrintString` (`KismetStringLibrary.Conv_DoubleToString` (`/Game/combat_system/Blueprints/Components/StatsComponent.GetCurrentStatValue` (`self.StatsComponent`) "NewEnumerator3")) true true (struct :`R` 0.192751 :`G` 1.0 :`A` 1.0))))

(event `/Game/combat_system/Blueprints/Interfaces/Targetable_BPI.OnTargeted`
  (params (isTargeted :type Boolean))
  (`SceneComponent.SetVisibility` (`self.LockOnWidget`) isTargeted false))

(fn `CanBeTargeted`
  (returns (`canBe Targeted` :type Boolean))
  (return (not (`/Game/combat_system/Blueprints/Components/StateManagerComponent.IsCurrentStateEqualToArray` (`self.StateManagerComponent`) (struct :`GameplayTags` (struct :`(TagName` "Character.State.Dead")))))))

(fn `UserConstructionScript`
  (`parent.UserConstructionScript`))