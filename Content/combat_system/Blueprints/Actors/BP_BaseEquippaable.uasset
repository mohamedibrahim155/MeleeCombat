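; Base equippable item actor for the combat system, tracking whether it is equipped and attaching itself to its owning character.
; Equipping sets the flag and snaps the item to the named attachment socket on the owner's Character mesh.
; Unequipping only clears the flag, without detaching.
; GetMesh returns the static mesh component when it has a mesh assigned, otherwise the skeletal one.
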(fn `AttachActor`
  (params (SocketName :type Name))
  (`self.K2_AttachToComponent` (`Character.Mesh` (cast `Character` (`self.GetOwner`) :!pure true)) SocketName "SnapToTarget" "SnapToTarget" "SnapToTarget"))

(fn `GetMesh`
  (returns (primitiveMesh :type "PrimitiveComponent Object Reference"))
  (bind _itemmesh (`self.itemMesh`))
  (`/Engine/EditorBlueprintResources/StandardMacros.IsValid` (`StaticMeshComponent.StaticMesh` _itemmesh)
    (:`Is Valid`
      (return _itemmesh))
    (:`Is Not Valid`
      (return (`self.itemSkeletonMesh`)))))

(fn `IsEquipped`
  (returns (bIsEquipped :type Boolean))
  (return (`self.bIsEquipped`)))

(fn `OnEquipped`
  (set `self.bIsEquipped` true)
  (`self.AttachActor` (`self.Attachment SocketName`)))

(fn `OnUnEquipped`
  (if (`self.bIsEquipped`)
    (set `self.bIsEquipped` false)))

(fn `SetIsEquippedState`
  (params (bIsEquipped :type Boolean))
  (set `self.bIsEquipped` bIsEquipped))

(fn `UserConstructionScript`)