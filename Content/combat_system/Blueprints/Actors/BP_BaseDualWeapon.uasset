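; Base Blueprint for dual-wielded weapons, adding an off-hand mesh and right-foot hit detection alongside the main weapon.
; Equipping and combat toggles snap the second mesh to the owner's hand socket in combat or its attach socket otherwise.
; Collision components for main weapon, off-hand and right foot are switched on and off by collision part.
; Their hits apply point damage to actors that can receive it, excluding the owner.
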(event `self.ToggleCombat`
  (params (`EnableCombat ?` :type Boolean))
  (`parent.ToggleCombat` `EnableCombat ?`)
  (`self.Attach Off-Hand Weapon` (select `bool` `EnableCombat ?` :`false` (`self.Second Weapon Attach Socket`) :`true` (`self.Second Weapon Hand Socket`))))

(event `self.MainWeaponCollisionComponent.OnHit`
  (params (hitInfo :type "HitResult Structure"))
  (bind (_bblockinghit _binitialoverlap _time _distance _location _impactpoint _normal _impactnormal _physmat _hitactor) (`GameplayStatics.BreakHitResult` hitInfo))
  (bind _returnvalue (`self.GetOwner`))
  (bind _returnvalue_2 (message `/Game/combat_system/Blueprints/Interfaces/ContinueAttack_BPI.CanReceiveDamage` _hitactor))
  (if (and _returnvalue_2 (!= _hitactor _returnvalue))
    (`GameplayStatics.ApplyPointDamage` _hitactor (`self.GetDamage`) (`self.GetActorForwardVector` _returnvalue) hitInfo (`self.GetInstigatorController`) _returnvalue)))

(event `self.RightFootColliderComponent.OnHit`
  (params (hitInfo :type "HitResult Structure"))
  (bind (_bblockinghit _binitialoverlap _time _distance _location _impactpoint _normal _impactnormal _physmat _hitactor) (`GameplayStatics.BreakHitResult` hitInfo))
  (bind _returnvalue (`self.GetOwner`))
  (bind _returnvalue_2 (message `/Game/combat_system/Blueprints/Interfaces/ContinueAttack_BPI.CanReceiveDamage` _hitactor))
  (if (and _returnvalue_2 (!= _hitactor _returnvalue))
    (`GameplayStatics.ApplyPointDamage` _hitactor (`self.GetDamage`) (`self.GetActorForwardVector` _returnvalue) hitInfo (`self.GetInstigatorController`) _returnvalue)))

(event `self.SecondWeaponCollisionComponent.OnHit`
  (params (hitInfo :type "HitResult Structure"))
  (bind _returnvalue (`self.GetOwner`))
  (bind (_bblockinghit _binitialoverlap _time _distance _location _impactpoint _normal _impactnormal _physmat _hitactor) (`GameplayStatics.BreakHitResult` hitInfo))
  (bind _returnvalue_2 (message `/Game/combat_system/Blueprints/Interfaces/ContinueAttack_BPI.CanReceiveDamage` _hitactor))
  (if (and _returnvalue_2 (!= _hitactor _returnvalue))
    (`GameplayStatics.ApplyPointDamage` _hitactor (`self.GetDamage`) (`self.GetActorForwardVector` _returnvalue) hitInfo (`self.GetInstigatorController`) _returnvalue)))

(fn `Activate Collision`
  (params (CollisionPart :type "/Game/combat_system/Blueprints/Enums/E_CollisionPart Enum" :default "NewEnumerator0"))
  (switch `/Game/combat_system/Blueprints/Enums/E_CollisionPart` CollisionPart
    (:`NewEnumerator0`
      (`/Game/combat_system/Blueprints/Components/CollisionComponent.EnableCollision` (`self.MainWeaponCollisionComponent`)))
    (:`NewEnumerator1`
      (`/Game/combat_system/Blueprints/Components/CollisionComponent.EnableCollision` (`self.SecondWeaponCollisionComponent`)))
    (:`NewEnumerator2`
      (`/Game/combat_system/Blueprints/Components/CollisionComponent.EnableCollision` (`self.RightFootColliderComponent`)))))

(fn `Attach Off-Hand Weapon`
  (params (socket :type Name))
  (`SceneComponent.K2_AttachToComponent` (`self.SecondMesh`) (`Character.Mesh` (cast `Character` (`self.GetOwner`) :!pure true)) socket "SnapToTarget" "SnapToTarget" "SnapToTarget" true))

(fn `Deactivate Collision`
  (params (CollisionPart :type "/Game/combat_system/Blueprints/Enums/E_CollisionPart Enum" :default "NewEnumerator0"))
  (switch `/Game/combat_system/Blueprints/Enums/E_CollisionPart` CollisionPart
    (:`NewEnumerator0`
      (`/Game/combat_system/Blueprints/Components/CollisionComponent.DisableCollision` (`self.MainWeaponCollisionComponent`)))
    (:`NewEnumerator1`
      (`/Game/combat_system/Blueprints/Components/CollisionComponent.DisableCollision` (`self.SecondWeaponCollisionComponent`)))
    (:`NewEnumerator2`
      (`/Game/combat_system/Blueprints/Components/CollisionComponent.DisableCollision` (`self.RightFootColliderComponent`)))))

(fn `OnEquipped`
  (`parent.OnEquipped`)
  (`/Game/combat_system/Blueprints/Components/CollisionComponent.SetMeshComponent` (`self.SecondWeaponCollisionComponent`) (`self.SecondMesh`))
  (`self.Attach Off-Hand Weapon` (select `bool` (`/Game/combat_system/Blueprints/Components/CombatComponent.IsCombatEnabled` (`self.CombatComponent`)) :`false` (`self.Second Weapon Attach Socket`) :`true` (`self.Second Weapon Hand Socket`)))
  (`/Game/combat_system/Blueprints/Components/CollisionComponent.SetMeshComponent` (`self.RightFootColliderComponent`) (`Character.Mesh` (cast `Character` (`self.GetOwner`) :!pure true)))
  (`/Game/combat_system/Blueprints/Components/CollisionComponent.AddActorsToAlwaysHitIgnoreList` (`self.SecondWeaponCollisionComponent`) (`self.GetOwner`))
  (`/Game/combat_system/Blueprints/Components/CollisionComponent.AddActorsToAlwaysHitIgnoreList` (`self.RightFootColliderComponent`) (`self.GetOwner`)))

(fn `UserConstructionScript`
  (`parent.UserConstructionScript`))