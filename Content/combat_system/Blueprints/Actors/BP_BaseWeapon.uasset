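; Base weapon actor that characters equip for combat, supplying action montages, stat costs and damage.
; On equip it registers with the owner's CombatComponent, updates the animation instance's attack type and attaches to hand or holster socket by combat state.
; Its collision component traces along the mesh, applying point damage to non-owner actors that accept it.
; Gameplay tags select montages, and the owner's current action looks up damage multiplier and cost.
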(event `self.MainWeaponCollisionComponent.OnHit`
  (params (hitInfo :type "HitResult Structure"))
  (bind (_bblockinghit _binitialoverlap _time _distance _location _impactpoint _normal _impactnormal _physmat _hitactor) (`GameplayStatics.BreakHitResult` hitInfo))
  (bind _returnvalue (`self.GetOwner`))
  (bind _returnvalue_2 (message `/Game/combat_system/Blueprints/Interfaces/ContinueAttack_BPI.CanReceiveDamage` _hitactor))
  (if (and _returnvalue_2 (!= _hitactor _returnvalue))
    (`GameplayStatics.ApplyPointDamage` _hitactor (`self.GetDamage`) (`self.GetActorForwardVector` _returnvalue) hitInfo (`self.GetInstigatorController`) _returnvalue)))

(event `SimulateWeaponPhysics`
  (bind _primitivemesh (`self.GetMesh`))
  (`PrimitiveComponent.SetCollisionProfileName` _primitivemesh "PhysicsActor" true)
  (`PrimitiveComponent.SetSimulatePhysics` _primitivemesh true))

(event `ToggleCombat`
  (params (`EnableCombat ?` :type Boolean))
  (`/Game/combat_system/Blueprints/Components/CombatComponent.SetCombatEnabled` (`self.CombatComponent`) `EnableCombat ?`)
  (`self.AttachActor` (select `bool` `EnableCombat ?` :`false` (`self.Attachment SocketName`) :`true` (`self.HandSocketName`))))

(fn `Activate Collision`
  (params (CollisionPart :type "/Game/combat_system/Blueprints/Enums/E_CollisionPart Enum" :default "NewEnumerator0"))
  (`/Game/combat_system/Blueprints/Components/CollisionComponent.EnableCollision` (`self.MainWeaponCollisionComponent`)))

(fn `Deactivate Collision`
  (params (CollisionPart :type "/Game/combat_system/Blueprints/Enums/E_CollisionPart Enum" :default "NewEnumerator0"))
  (`/Game/combat_system/Blueprints/Components/CollisionComponent.DisableCollision` (`self.MainWeaponCollisionComponent`)))

(fn `Get Action Montages`
  (params (actionState :type "GameplayTag Structure"))
  (returns (Montages :type "Array of AnimMontage Object Reference"))
  (`|SwitchGameplayTag` actionState
    (:`Character.Action.Attack.Light Attack`
      (return (`self.LightAttackMontages`)))
    (:`Character.Action.Attack.Heavy Attack`
      (return (`self.Heavy Attack`)))
    (:`Character.Action.Attack.Falling Attack`
      (return (`self.Falling Attack`)))
    (:`Character.Action.Attack.Sprint Attack`
      (return (`self.Sprint Attack`)))
    (:`Character.Action.Attack.Charged Attack`
      (return (`self.Charged Attack`)))
    (:`Character.Action.Dodge`
      (return (`self.DodgeMontages`)))
    (:`Character.Action.Enter Combat`
      (return (`|MakeArray` (`self.EnterMontage`))))
    (:`Character.Action.Exit Combat`
      (return (`|MakeArray` (`self.ExitMontage`))))))

(fn `GetDamage`
  (returns (Value :type "Float (double-precision)"))
  (bind _statemanagercomponent (`self.StateManagerComponent`)
    (:`then`
      (bind _returnvalue (* (`self.damange`) (`BlueprintMapLibrary.Map_Find` (`self.DamageMultiplier`) (`/Game/combat_system/Blueprints/Components/StateManagerComponent.GetCurrentAction` _statemanagercomponent))))
      (return (`KismetMathLibrary.FClamp` _returnvalue 1.0 _returnvalue)))
    (:`else`
      (return (`self.damange`)))))

(fn `GetStatCostForAction`
  (returns (Value :type "Float (double-precision)"))
  (bind _statemanagercomponent (`self.StateManagerComponent`)
    (:`then`
      (return (`BlueprintMapLibrary.Map_Find` (`self.ActionStatCost`) (`/Game/combat_system/Blueprints/Components/StateManagerComponent.GetCurrentAction` _statemanagercomponent))))
    (:`else`
      (return 0.0))))

(fn `GetWeaponState`
  (returns (WeaponState :type "GameplayTag Structure"))
  (return (`/Game/combat_system/Blueprints/Components/StateManagerComponent.GetCurrentState` (`self.WeaponStateManager`))))

(fn `OnEquipped`
  (bind _returnvalue (`self.GetOwner`))
  (bind _mainweaponcollisioncomponent (`self.MainWeaponCollisionComponent`))
  (`parent.OnEquipped`)
  (`/Game/combat_system/Blueprints/Components/StateManagerComponent.SetState` (`self.WeaponStateManager`) (struct :`TagName` "Weapon.State.Equipped"))
  (set `self.CombatComponent` (`self.GetComponentByClass` _returnvalue "/Game/combat_system/Blueprints/Components/CombatComponent.CombatComponent_C"))
  (set `self.StateManagerComponent` (`self.GetComponentByClass` _returnvalue "/Game/combat_system/Blueprints/Components/StateManagerComponent.StateManagerComponent_C"))
  (`self.AttachActor` (select `bool` (`/Game/combat_system/Blueprints/Components/CombatComponent.IsCombatEnabled` (`self.CombatComponent`)) :`false` (`self.Attachment SocketName`) :`true` (`self.HandSocketName`)))
  (`/Game/combat_system/Blueprints/Components/CombatComponent.SetMainWeapon` (`self.CombatComponent`) self)
  (message `/Game/combat_system/Blueprints/Interfaces/AttackAnimation_BPI.UpdateAnimationBasedOnAttackType` (`SkeletalMeshComponent.GetAnimInstance` (`Character.Mesh` (cast `/Game/combat_system/Blueprints/BP_CombatCharacter` _returnvalue :!pure true))) (`self.eCombatType`))
  ;[1 1 1] SetUp for collision trace
  (`/Game/combat_system/Blueprints/Components/CollisionComponent.SetMeshComponent` _mainweaponcollisioncomponent (`self.GetMesh`))
  (`/Game/combat_system/Blueprints/Components/CollisionComponent.AddActorsToAlwaysHitIgnoreList` _mainweaponcollisioncomponent (`self.GetOwner`)))

(fn `OnUnEquipped`
  (`parent.OnUnEquipped`)
  (`/Game/combat_system/Blueprints/Components/StateManagerComponent.SetState` (`self.WeaponStateManager`) (struct :`TagName` "Weapon.State.Unequipped")))

(fn `UserConstructionScript`
  (`parent.UserConstructionScript`))