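; Actor stats component for the combat system, tracking current values against base and max definitions for stats such as Health, Stamina and Armour.
; Stat modifications clamp between zero and max, then fire a value-change notification.
; TakeDamage scales incoming damage by damage/(damage+Armour), intending a minimum of one.
; Spending stamina stops regeneration, which a retriggerable delay restarts as a looping timer until full.
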(event `StartRegen`
  (params (Stat :type "/Game/combat_system/Blueprints/Enums/E_Stats Enum" :default "NewEnumerator0"))
  (switch `/Game/combat_system/Blueprints/Enums/E_Stats` Stat
    (:`NewEnumerator2`
      (`KismetSystemLibrary.K2_ClearTimer` null "RegenerateStamina")
      (`KismetSystemLibrary.RetriggerableDelay` 1.2)
      (`KismetSystemLibrary.K2_SetTimer` null "RegenerateStamina" 0.1 true))))

(fn `AddBaseStatsBaseValue`
  (params (Stat :type "/Game/combat_system/Blueprints/Enums/E_Stats Enum" :default "NewEnumerator0") (Value :type "Float (double-precision)"))
  (bind _structout (setmembers `/Game/combat_system/Blueprints/Structs/F_BaseStat` :`StructRef` (`BlueprintMapLibrary.Map_Find` (`self.BaseStats`) (`local.Stat`)) :`BaseValue` Value))
  (`BlueprintMapLibrary.Map_Add` (`self.BaseStats`) (`local.Stat`) _structout))

(fn `AddBaseStatsMaxValue`
  (params (Stat :type "/Game/combat_system/Blueprints/Enums/E_Stats Enum (by ref)") (Value :type "Float (double-precision)"))
  (bind _structout (setmembers `/Game/combat_system/Blueprints/Structs/F_BaseStat` :`StructRef` (`BlueprintMapLibrary.Map_Find` (`self.BaseStats`) (`local.Stat`)) :`MaxValue` Value))
  (`BlueprintMapLibrary.Map_Add` (`self.BaseStats`) (`local.Stat`) _structout))

(fn `Get Stats Base Value`
  (params (Stat :type "/Game/combat_system/Blueprints/Enums/E_Stats Enum" :default "NewEnumerator0"))
  (returns (`Base Value` :type "Float (double-precision)"))
  (return (break `/Game/combat_system/Blueprints/Structs/F_BaseStat` (`BlueprintMapLibrary.Map_Find` (`self.BaseStats`) Stat))))

(fn `GetCurrentStatValue`
  (params (stat :type "/Game/combat_system/Blueprints/Enums/E_Stats Enum" :default "NewEnumerator0"))
  (returns (returrnValue :type "Float (double-precision)"))
  (return (`BlueprintMapLibrary.Map_Find` (`self.CurrentStat`) stat)))

(fn `GetStatsMaxValue`
  (params (stat :type "/Game/combat_system/Blueprints/Enums/E_Stats Enum" :default "NewEnumerator0"))
  (returns (`Max Value` :type "Float (double-precision)"))
  (return (`.MaxValue_4_7D7F5A5A4044C4B43528DD9F57227BA9` (break `/Game/combat_system/Blueprints/Structs/F_BaseStat` (`BlueprintMapLibrary.Map_Find` (`self.BaseStats`) stat)))))

(fn `IntialiseStats`
  (bind _keys (`BlueprintMapLibrary.Map_Keys` (`self.BaseStats`)))
  (for _array_element _keys
    (`self.SetCurrentStatValue` _array_element (break `/Game/combat_system/Blueprints/Structs/F_BaseStat` (`BlueprintMapLibrary.Map_Find` (`self.BaseStats`) _array_element)))))

(fn `ModifyCurrentStatValue`
  (params (stat :type "/Game/combat_system/Blueprints/Enums/E_Stats Enum" :default "NewEnumerator0") (value :type "Float (double-precision)") (bShouldRegenerate :type Boolean :default false))
  (locals (L_Value :type "Float (double-precision)"))
  (if (!= value 0.0)
    (bind _output_get (set `local.L_Value` (+ (`self.GetCurrentStatValue` (`local.stat`)) (`local.value`))))
    (bind _output_get_2 (set `local.L_Value` (`KismetMathLibrary.FClamp` _output_get 0.0 (`self.GetStatsMaxValue` (`local.stat`)))))
    (`self.SetCurrentStatValue` (`local.stat`) _output_get_2)
    (if (`local.bShouldRegenerate`)
      (`self.StartRegen` (`local.stat`))
      (return))))

(fn `ModifyStamina`
  (params (inStaminaCost :type "Float (double-precision)"))
  (`self.ModifyCurrentStatValue` "NewEnumerator2" (* inStaminaCost -1.0) true))

(fn `RegenerateStamina`
  (locals (L_Stamina :type "Float (double-precision)"))
  (`self.SetCurrentStatValue` "NewEnumerator2" (`KismetMathLibrary.FClamp` (+ (`self.GetCurrentStatValue` "NewEnumerator2") (`self.RegenRate`)) 0.0 (`self.GetStatsMaxValue` "NewEnumerator2")))
  (if (>= (`self.GetCurrentStatValue` "NewEnumerator2") (`self.GetStatsMaxValue` "NewEnumerator2"))
    (`KismetSystemLibrary.K2_ClearTimer` null "RegenerateStamina")))

(fn `SetCurrentStatValue`
  (params (Stat :type "/Game/combat_system/Blueprints/Enums/E_Stats Enum" :default "NewEnumerator0") (Value :type "Float (double-precision) (by ref)"))
  (`BlueprintMapLibrary.Map_Add` (`self.CurrentStat`) Stat Value)
  (`self.OnStatsValueChange` (`local.Stat`) (`local.Value`)))

(fn `TakeDamage`
  (params (inDamage :type "Float (double-precision)"))
  (locals (damageMultiplyer :type "Float (double-precision)") (damageAmount :type "Float (double-precision)"))
  (bind _indamage (`local.inDamage`))
  (bind _output_get (set `local.damageMultiplyer` (/ _indamage (+ _indamage (`self.GetCurrentStatValue` "NewEnumerator3")))))
  (bind _returnvalue (* _output_get (`local.inDamage`)))
  (set `local.damageAmount` (`KismetMathLibrary.FClamp` _returnvalue 1.0 _returnvalue))
  (`self.ModifyCurrentStatValue` "NewEnumerator1" (* (`local.damageAmount`) -1.0)))