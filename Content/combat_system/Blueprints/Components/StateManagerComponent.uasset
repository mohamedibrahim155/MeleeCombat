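; StateManagerComponent is a combat system component that tracks its owner's current state and current action as two separate values.
; Setters ignore unchanged values and fire notifications around each change, while query functions return or compare the values, including against arrays.
; ResetState returns only the state to a default enum entry.
; SetCurrentAction fires Begin with the outgoing action and Exit with the incoming one, the reverse of SetState's exit-then-enter order.
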(fn `GetCurrentAction`
  (returns (currentActionState :type "/Game/combat_system/Blueprints/Enums/E_PlayerAction Enum"))
  (return (`self.currentActionState`)))

(fn `GetCurrentState`
  (returns (currentState :type "/Game/combat_system/Blueprints/Enums/E_PlayerState Enum"))
  (return (`self.currentState`)))

(fn `IsCurrentAction`
  (params (StateCheck :type "/Game/combat_system/Blueprints/Enums/E_PlayerAction Enum" :default "NewEnumerator0"))
  (returns (ReturnValue :type Boolean))
  (return (`|EnumEquality` StateCheck (`self.currentActionState`))))

(fn `IsCurrentActionContainsAny`
  (params (actionList :type "Array of /Game/combat_system/Blueprints/Enums/E_PlayerAction Enum"))
  (returns (ReturnValue :type Boolean))
  (return (`KismetArrayLibrary.Array_Contains` actionList (`self.currentActionState`))))

(fn `IsCurrentStateEqualToArray`
  (params (States :type "Array of /Game/combat_system/Blueprints/Enums/E_PlayerState Enum"))
  (returns (ReturnValue :type Boolean))
  (return (`KismetArrayLibrary.Array_Contains` States (`self.currentState`))))

(fn `ResetState`
  (`self.SetState` "NewEnumerator0"))

(fn `SetCurrentAction`
  (params (`new Action` :type "/Game/combat_system/Blueprints/Enums/E_PlayerAction Enum" :default "NewEnumerator0"))
  (bind _currentactionstate (`self.currentActionState`))
  (if (`|EnumInequality` _currentactionstate `new Action`)
    (`self.OnActionBegin` _currentactionstate)
    (bind _output_get (set `self.currentActionState` (`local.new Action`)))
    (`self.OnActionExit` _output_get)))

(fn `SetState`
  (params (newState :type "/Game/combat_system/Blueprints/Enums/E_PlayerState Enum" :default "NewEnumerator0"))
  (if (`|EnumInequality` newState (`self.currentState`))
    (`self.OnStateExit` (`self.currentState`))
    (bind _output_get (set `self.currentState` (`local.newState`)))
    (`self.OnStateEnter` _output_get)))