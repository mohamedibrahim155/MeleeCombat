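; Combat component that tracks the owner's main weapon, combat-enabled state and attack progress.
; Setting a new main weapon first calls OnUnEquipped on any valid current one and destroys it, then stores the replacement.
; Changing the combat state broadcasts it through the OnToggleCombat dispatcher, and ResetAttack clears the saved-attack flag and attack count.
; The event graph is unused, so all behavior runs through functions called from outside.
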(fn `GetMainWeapon`
  (returns (`Main Weapon` :type "/Game/combat_system/Blueprints/Actors/BP_BaseWeapon Object Reference"))
  (return (`self.Main Weapon`)))

(fn `IsCombatEnabled`
  (returns (bIsCombatEnabled :type Boolean))
  (return (`self.bIsCombatEnabled`)))

(fn `ResetAttack`
  (set `self.bIsAttackSaved` false)
  (set `self.AttackCount` 0))

(fn `SetCombatEnabled`
  (params (bIsCombatEnabled :type Boolean))
  (set `self.bIsCombatEnabled` bIsCombatEnabled)
  (`self.OnToggleCombat` (`self.bIsCombatEnabled`)))

(fn `SetMainWeapon`
  (params (newWeapon :type "/Game/combat_system/Blueprints/Actors/BP_BaseWeapon Object Reference"))
  (bind _main_weapon (`self.Main Weapon`))
  (`|ExecutionSequence`
    (:`then_0`
      (`/Engine/EditorBlueprintResources/StandardMacros.IsValid` _main_weapon
        (:`Is Valid`
          (`/Game/combat_system/Blueprints/Actors/BP_BaseEquippaable.OnUnEquipped` _main_weapon)
          (`Actor.K2_DestroyActor` _main_weapon))))
    (:`then_1`
      (set `self.Main Weapon` (`local.newWeapon`)))))