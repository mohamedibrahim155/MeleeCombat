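; Combat component that detects melee-style hits by sweeping a sphere trace between two sockets on an assigned mesh.
; While collision is enabled, Tick traces each frame and fires CallOnHit once per newly hit actor.
; Hit actors join an ignore list, cleared on each enable and editable externally, preventing repeat hits within one activation.
; The last hit result and hit actor are stored for querying.
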(event `EnableCollision`
  (`self.ClearHitActors`)
  (set `self.bIsCollisionEnabled` true))

(event `DisableCollision`
  (set `self.bIsCollisionEnabled` false))

(event `ClearHitActors`
  (`KismetArrayLibrary.Array_Clear` (`self.AlreadyHitActors`)))

(event `self.ReceiveTick`
  (params (DeltaSeconds :type "Float (single-precision)"))
  (if (`self.bIsCollisionEnabled`)
    (`self.CollisionTrace`)))

(event `CollisionTrace`
  (bind _mesh (`self.Mesh`))
  (bind _outhits (`KismetSystemLibrary.SphereTraceMultiForObjects` (`SceneComponent.GetSocketLocation` _mesh (`self.StartTrace Socket name`)) (`SceneComponent.GetSocketLocation` _mesh (`self.EndTrace Socket name`)) (`self.TraceRadius`) (`self.Object Types`) false (`self.AlreadyHitActors`) (`self.Draw Debug Type`) true (struct :`R` 1.0 :`A` 1.0) (struct :`G` 1.0 :`A` 1.0) 1.0))
  (for _array_element _outhits
    (bind _output_get (set `self.LasrHit` _array_element))
    (bind (_bblockinghit _binitialoverlap _time _distance _location _impactpoint _normal _impactnormal _physmat _hitactor) (`GameplayStatics.BreakHitResult` _output_get))
    (if (not (`KismetArrayLibrary.Array_Contains` (`self.AlreadyHitActors`) _hitactor))
      (set `self.HitActor` _hitactor)
      (`KismetArrayLibrary.Array_Add` (`self.AlreadyHitActors`) _hitactor)
      (`self.OnHit` self (`self.LasrHit`)))))

(fn `AddActorsToIgnoreList`
  (params (actor :type "Actor Object Reference (by ref)"))
  (`KismetArrayLibrary.Array_AddUnique` (`self.AlreadyHitActors`) actor))

(fn `GetHitActor`
  (returns (HitActor :type "Actor Object Reference"))
  (return (`self.HitActor`)))

(fn `GetLastHit`
  (returns (LasrHit :type "HitResult Structure"))
  (return (`self.LasrHit`)))

(fn `IsCollisionEnabled`
  (returns (bIsCollisionEnabled :type Boolean))
  (return (`self.bIsCollisionEnabled`)))

(fn `RemoveActorsToIngoreList`
  (params (actor :type "Actor Object Reference (by ref)"))
  (`KismetArrayLibrary.Array_RemoveItem` (`self.AlreadyHitActors`) actor))

(fn `SetMeshComponent`
  (params (Mesh :type "PrimitiveComponent Object Reference"))
  (set `self.Mesh` Mesh))