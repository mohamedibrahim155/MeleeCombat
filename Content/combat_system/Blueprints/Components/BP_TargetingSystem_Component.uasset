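; Lock-on targeting component for a Character that keeps the view turned toward a targeted enemy or other Targetable_BPI actor.
; Locking sphere-traces along the camera's forward vector, checks targetability and range, and notifies the target through the interface.
; While locked, Tick interpolates control pitch and yaw toward the target, unlocking when it becomes invalid.
; Rotation switches between orient-to-camera and orient-to-movement based on combat, lock and speed mode.
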(event `self.ReceiveBeginPlay`
  ;[1 1 1] Initializations
  (bind _ascharacter (cast `Character` (`self.GetOwner`)))
  (bind _output_get (set `self.Owner Character` _ascharacter))
  (set `self.Owner Controller` (`Pawn.GetController` _output_get))
  (set `self.FollowCamera` (`Actor.GetComponentByClass` _output_get "/Script/Engine.CameraComponent")))

(event `self.ReceiveTick`
  (params (DeltaSeconds :type "Float (single-precision)"))
  (if (`self.isLocked`)
    (`self.UpdateRotationBasedOnTarget`)))

(event `EnableLock`
  (bind (_found_success _found_actor) (`self.FindTarget`))
  (if (and _found_success (`self.Can Target Actor` _found_actor))
    (`self.SetFoundActor` _found_actor)
    (`self.SetLockedState` true)
    (`self.UpdateRotationMode`)))

(event `DisableLock`
  (`self.SetLockedState` false)
  (`self.SetFoundActor` null)
  (`self.Set Rotation Mode` "NewEnumerator1")
  (`self.UpdateRotationMode`))

(event `ToggleLocking`
  (if (not (`self.IsTargetLocked`))
    (`self.EnableLock`)
    (else
      (`self.DisableLock`))))

(fn `Can Target Actor`
  (params (`in actor` :type "Actor Object Reference"))
  (returns (ReturnValue :type Boolean))
  (`/Engine/EditorBlueprintResources/StandardMacros.IsValid` `in actor`
    (:`Is Valid`
      (bind _canbe_targeted (message `/Game/combat_system/Blueprints/Interfaces/Targetable_BPI.CanBeTargeted` `in actor`))
      (return (and _canbe_targeted (< (`Actor.GetDistanceTo` (`self.GetOwner`) (`local.in actor`)) (`self.RayDistance`)))))
    (:`Is Not Valid`
      (return false))))

(fn `FindTarget`
  (returns (`Found Success` :type Boolean) (`Found Actor` :type "Actor Object Reference"))
  (bind (_outhit _returnvalue) (`KismetSystemLibrary.SphereTraceSingleForObjects` (`Actor.K2_GetActorLocation` (`self.Owner Character`)) (+ (* (`SceneComponent.GetForwardVector` (`self.FollowCamera`)) (`self.RayDistance`)) (`Actor.K2_GetActorLocation` (`self.Owner Character`))) (`self.SphereTraceRadius`) (`self.Object Types`) false (`|MakeArray` (`self.Owner Character`) :!type "Actor Object Reference") (`self.Draw Debug Type`) true (struct :`R` 1.0 :`A` 1.0) (struct :`G` 1.0 :`A` 1.0) 2.0))
  (bind (_bblockinghit _binitialoverlap _time _distance _location _impactpoint _normal _impactnormal _physmat _hitactor) (`GameplayStatics.BreakHitResult` _outhit))
  (if (and _returnvalue (`KismetSystemLibrary.IsValid` _hitactor))
    (if (`KismetSystemLibrary.DoesImplementInterface` _hitactor "/Game/combat_system/Blueprints/Interfaces/Targetable_BPI.Targetable_BPI_C")
      (return true _hitactor)
      (else
        (return false null)))
    (else
      (return false null))))

(fn `GetFoundActor`
  (returns (`Found Actor` :type "Actor Object Reference"))
  (return (`self.Targeting Actor`)))

(fn `IsTargetLocked`
  (returns (isLocked :type Boolean))
  (return (`self.isLocked`)))

(fn `Set Rotation Mode`
  (params (rotationMode :type "/Game/combat_system/Blueprints/Enums/E_RotationMode Enum" :default "NewEnumerator0"))
  (bind _owner_character (`self.Owner Character`))
  (bind _charactermovement (`Character.CharacterMovement` _owner_character))
  (bind _output_get (set `self.Rotation Mode` rotationMode))
  (switch `/Game/combat_system/Blueprints/Enums/E_RotationMode` _output_get
    (:`NewEnumerator0`
      (set `Pawn.bUseControllerRotationYaw` true _owner_character)
      (set `CharacterMovementComponent.bUseControllerDesiredRotation` true _charactermovement)
      (set `CharacterMovementComponent.bOrientRotationToMovement` false _charactermovement))
    (:`NewEnumerator1`
      (set `Pawn.bUseControllerRotationYaw` false _owner_character)
      (set `CharacterMovementComponent.bUseControllerDesiredRotation` false _charactermovement)
      (set `CharacterMovementComponent.bOrientRotationToMovement` true _charactermovement))))

(fn `SetFoundActor`
  (params (`Found Actor` :type "Actor Object Reference"))
  (set `self.Targeting Actor` `Found Actor`))

(fn `SetLockedState`
  (params (`Can Lock` :type Boolean))
  (set `self.isLocked` `Can Lock`)
  (bind _targeting_actor (`self.Targeting Actor`)
    (:`then`
      (message `/Game/combat_system/Blueprints/Interfaces/Targetable_BPI.OnTargeted` _targeting_actor (`self.isLocked`)))
    (:`else`)))

(fn `UpdateRotationBasedOnTarget`
  (bind _returnvalue (`Actor.K2_GetActorRotation` (`self.Owner Controller`)))
  (if (and (`KismetSystemLibrary.IsValid` (`self.Owner Character`)) (`KismetSystemLibrary.IsValid` (`self.Targeting Actor`)) (`self.Can Target Actor` (`self.Targeting Actor`)))
    (`Controller.SetControlRotation` (`self.Owner Controller`) (`KismetMathLibrary.MakeRotator` (.roll _returnvalue) (.pitch (`KismetMathLibrary.RInterpTo` _returnvalue (`KismetMathLibrary.FindLookAtRotation` (`Actor.K2_GetActorLocation` (`self.GetOwner`)) (- (`Actor.K2_GetActorLocation` (`self.Targeting Actor`)) (0.0 0.0 100.0))) (`GameplayStatics.GetWorldDeltaSeconds`) (`self.Rotaion Speed`))) (.yaw (`KismetMathLibrary.RInterpTo` _returnvalue (`KismetMathLibrary.FindLookAtRotation` (`Actor.K2_GetActorLocation` (`self.GetOwner`)) (- (`Actor.K2_GetActorLocation` (`self.Targeting Actor`)) (0.0 0.0 100.0))) (`GameplayStatics.GetWorldDeltaSeconds`) (`self.Rotaion Speed`)))))
    (else
      (`self.DisableLock`))))

(fn `UpdateRotationMode`
  (`/Engine/EditorBlueprintResources/StandardMacros.IsValid` (`self.Owner Combat Component`)
    (:`Is Valid`
      _)
    (:`Is Not Valid`
      (set `self.Owner Combat Component` (`Actor.GetComponentByClass` (`self.Owner Character`) "/Game/combat_system/Blueprints/Components/CombatComponent.CombatComponent_C"))))
  (bind _speedmode (message `/Game/combat_system/Blueprints/Interfaces/ContinueAttack_BPI.GetMovementSpeedMode` (`self.Owner Character`)))
  (`self.Set Rotation Mode` (select `bool` (and (`/Game/combat_system/Blueprints/Components/CombatComponent.IsCombatEnabled` (`self.Owner Combat Component`)) (`|EnumInequality` _speedmode "NewEnumerator1") (`self.IsTargetLocked`)) :`false` "NewEnumerator1" :`true` "NewEnumerator0" :!type "/Game/combat_system/Blueprints/Enums/E_RotationMode Enum")))

(fn `UpdateTargetRotationBasedNear`)